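; Bomber biplane pawn for a multiplayer game, which drops bombs and takes hits from mecha projectiles.
; On BeginPlay it registers as the game mode's Bomber and switches the default pawn to FirstPersonCharacter for the next spawn.
; Fire spawns a bomb below the plane, while body or wing overlaps with a MechaProjectile decrement the bomber health held in the game mode.
; Banking and turning logic remains only in unexecuted legacy functions.
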(event `self.ReceiveBeginPlay`
  ;[1 0.3388 0] BeginPlay : Change le prochain pawn à être spawné
  (bind _asbp_multiplayer_game_mode (cast `/Game/Blueprints/BP_Luc/BP_MultiplayerGameMode` (`GameplayStatics.GetGameMode`)))
  (set `GameModeBase.DefaultPawnClass` "/Game/Blueprints/JoffreyZ/Resistant/FirstPersonCharacter.FirstPersonCharacter_C" _asbp_multiplayer_game_mode)
  (set `/Game/Blueprints/BP_Luc/BP_MultiplayerGameMode.Bomber` self _asbp_multiplayer_game_mode))

(event `InputAction|Fire`
  (params (Key :type "Key Structure"))
  ;[1 0 0] SpawnProjectile
  (:`Pressed`
    (`self.SpawnProjectile`)))

(event `SpawnProjectile`
  ;[0.9131 0 1] Créer un projectile sur le serveur
  (`|SpawnActorFromClass` "/Game/Blueprints/BP_Luc/BP_BombeProjectile.BP_BombeProjectile_C" (`self.ProjectileSpawnTransform`) "Undefined" "OverrideRootScale" null null))

(event `ServerDame`
  (params (Obus :type "Actor Object Reference"))
  ;[1 1 1] Reduction de Santé biplan
  (cast `/Game/Blueprints/JoffreyZ/Mecha/MechaProjectile` Obus)
  (bind _asbp_multiplayer_game_mode (cast `/Game/Blueprints/BP_Luc/BP_MultiplayerGameMode` (`GameplayStatics.GetGameMode`)))
  (set `/Game/Blueprints/BP_Luc/BP_MultiplayerGameMode.SanteBomber` (- (`/Game/Blueprints/BP_Luc/BP_MultiplayerGameMode.SanteBomber` _asbp_multiplayer_game_mode) 1) _asbp_multiplayer_game_mode))

(event `self.Body.OnComponentBeginOverlap`
  (params (OverlappedComponent :type "PrimitiveComponent Object Reference") (OtherActor :type "Actor Object Reference") (OtherComp :type "PrimitiveComponent Object Reference") (OtherBodyIndex :type Integer) (bFromSweep :type Boolean) (SweepResult :type "HitResult Structure (by ref)"))
  ;[1 1 1] Reduction de Santé biplan
  (`self.ServerDame` OtherActor))

(event `self.Wings.OnComponentBeginOverlap`
  (params (OverlappedComponent :type "PrimitiveComponent Object Reference") (OtherActor :type "Actor Object Reference") (OtherComp :type "PrimitiveComponent Object Reference") (OtherBodyIndex :type Integer) (bFromSweep :type Boolean) (SweepResult :type "HitResult Structure (by ref)"))
  ;[1 1 1] Reduction de Santé biplan
  (`self.ServerDame` OtherActor))

(fn `Old`
  (params (InputPin :type "Float (double-precision)")))

(fn `Old 1`
  (set `PlayerController.InputYawScale` (/ (`KismetMathLibrary.Abs` (`self.RollAngle_0`)) 100.0) (`GameplayStatics.GetPlayerController` 0))
  (`self.AddControllerYawInput` (`self.GetInputAxisValue`)))

(fn `ProjectileSpawnTransform`
  (returns (ReturnValue :type "Transform Structure"))
  (bind _returnvalue (`self.GetTransform`))
  (return (`KismetMathLibrary.MakeTransform` (`KismetMathLibrary.MakeVector` (.x (.location _returnvalue)) (.y (.location _returnvalue)) (- (.z (.location _returnvalue)) 400.0)) (.rotation _returnvalue) (.scale _returnvalue))))

(fn `UserConstructionScript`)