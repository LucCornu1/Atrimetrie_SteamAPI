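; BuildingBox_BP is a bombing objective that adds to the game's destroyed-objective count when a bomb hits it.
; On BeginPlay it finds and stores the BP_MultiplayerGameMode actor.
; When a BP_BombeProjectile overlaps DetectBomb, it destroys the bomb and the MeshReference actor, increments ObjectivesDestroyed on the game mode, prints debug text, then destroys itself.
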(event `self.ReceiveBeginPlay`
  ;[1 1 1] Get plane reference
  (bind _returnvalue (`GameplayStatics.GetActorOfClass` "/Game/Blueprints/BP_Luc/BP_MultiplayerGameMode.BP_MultiplayerGameMode_C")))

(event `self.DetectBomb.OnComponentBeginOverlap`
  (params (OverlappedComponent :type "PrimitiveComponent Object Reference") (OtherActor :type "Actor Object Reference") (OtherComp :type "PrimitiveComponent Object Reference") (OtherBodyIndex :type Integer) (bFromSweep :type Boolean) (SweepResult :type "HitResult Structure (by ref)"))
  ;[1 1 1] Building & points
  (bind _asbp_bombe_projectile (cast `/Game/Blueprints/BP_Luc/BP_BombeProjectile` OtherActor))
  (`self.K2_DestroyActor` _asbp_bombe_projectile)
  (`self.K2_DestroyActor` (`self.MeshReference`))
  (`KismetSystemLibrary.PrintString` "+1" true true (struct :`R` 1.0 :`B` 0.007034 :`A` 1.0))
  (set `/Game/Blueprints/BP_Luc/BP_MultiplayerGameMode.ObjectivesDestroyed` (+ (`/Game/Blueprints/BP_Luc/BP_MultiplayerGameMode.ObjectivesDestroyed` (stale `self.ReceiveBeginPlay` _returnvalue)) 1) (stale `self.ReceiveBeginPlay` _returnvalue))
  (`KismetSystemLibrary.PrintString` (`KismetStringLibrary.Conv_IntToString` (`/Game/Blueprints/BP_Luc/BP_MultiplayerGameMode.ObjectivesDestroyed` (stale `self.ReceiveBeginPlay` _returnvalue))) true true (struct :`R` 1.0 :`B` 0.006995 :`A` 1.0))
  (`self.K2_DestroyActor`))

(fn `UserConstructionScript`)